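; BP_office_door is an interactive swinging door that opens on the F key and closes when an overlap with its trigger ends.
; DoorTrigger overlap enables player 0 input and shows two text renders, without checking which actor overlaps.
; F plays the DoorSwinging timeline, which drives Hinge yaw and hides the texts as it updates.
; End overlap disables input, hides the texts and reverses the timeline.
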(event OnComponentBeginOverlap(DoorTrigger)
  (params (OverlappedComponent :type Primitive%20Component%20Object%20Reference) (OtherActor :type Actor%20Object%20Reference) (OtherComp :type Primitive%20Component%20Object%20Reference) (OtherBodyIndex :type Integer) (bFromSweep :type Boolean) (SweepResult :type Hit%20Result%20Structure%20%28by%20ref%29))
  (Input|EnableInput (Game|GetPlayerController 0))
  (Rendering|SetVisibility (Variables|Default|GetTextRender1) true false))

(event OnComponentEndOverlap(DoorTrigger)
  (params (OverlappedComponent :type Primitive%20Component%20Object%20Reference) (OtherActor :type Actor%20Object%20Reference) (OtherComp :type Primitive%20Component%20Object%20Reference) (OtherBodyIndex :type Integer))
  (Input|DisableInput (Game|GetPlayerController 0))
  (Rendering|SetVisibility (Variables|Default|GetTextRender1) false false)
  (bind _doorangle (Timeline|DoorSwinging Reverse)
    (:Update
      (Transformation|SetRelativeRotation (Variables|Default|GetHinge) (Math|Rotator|MakeRotator 0.0 0.0 _doorangle) false false)
      (Rendering|SetVisibility (Variables|Default|GetTextRender1) false false))))

(event Input|KeyboardEvents|F
  (params (Key :type Key%20Structure :default "None"))
  (:Pressed
    (bind _doorangle (Timeline|DoorSwinging Play)
      (:Update
        (Transformation|SetRelativeRotation (Variables|Default|GetHinge) (Math|Rotator|MakeRotator 0.0 0.0 _doorangle) false false)
        (Rendering|SetVisibility (Variables|Default|GetTextRender1) false false)))))

(fn ConstructionScript)