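; BP_filled_mug is an interactive mug prop whose mesh material gets a random color on BeginPlay.
; Its trigger overlap shows two text renders and enables player 0 input, reversing both on exit, without checking which actor overlaps.
; While input is enabled, pressing F re-randomizes the Color parameter using a random unit vector, without the random brightness scale applied at BeginPlay.
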(event OnComponentBeginOverlap(Trigger)
  (params (OverlappedComponent :type Primitive%20Component%20Object%20Reference) (OtherActor :type Actor%20Object%20Reference) (OtherComp :type Primitive%20Component%20Object%20Reference) (OtherBodyIndex :type Integer) (bFromSweep :type Boolean) (SweepResult :type Hit%20Result%20Structure%20%28by%20ref%29))
  ;[1 1 1] On Overlap - show text and enable input
  (Input|EnableInput (Game|GetPlayerController 0))
  (Rendering|SetVisibility (Variables|Default|GetTextRender) true false))

(event OnComponentEndOverlap(Trigger)
  (params (OverlappedComponent :type Primitive%20Component%20Object%20Reference) (OtherActor :type Actor%20Object%20Reference) (OtherComp :type Primitive%20Component%20Object%20Reference) (OtherBodyIndex :type Integer))
  ;[1 1 1] End Overlap - hide text and disable input
  (Input|DisableInput (Game|GetPlayerController 0))
  (Rendering|SetVisibility (Variables|Default|GetTextRender1) false false))

(event EventBeginPlay
  ;[1 1 1] Random color at begin
  (Rendering|Material|SetVectorParameterValueonMaterials (Variables|Debug|GetStaticMeshComponent) "Color" (* (Math|Random|RandomUnitVector) (Math|Random|RandomFloatinRange 0.0 1.0))))

(event Input|KeyboardEvents|F
  (params (Key :type Key%20Structure :default "None"))
  ;[1 1 1] When F is pressed - random color
  (:Pressed
    (Rendering|Material|SetVectorParameterValueonMaterials (Variables|Debug|GetStaticMeshComponent) "Color" (Math|Random|RandomUnitVector))))

(fn ConstructionScript)